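; Anim notify that plays a surface-specific footstep sound when an animation reaches it.
; It traces 200 units down from the owning actor on Visibility and switches on the hit's physical surface to choose a grass, metal, wood, water or default sound.
; Each sound gets randomized pitch, with volume also randomized for water.
; No play call uses the hit or actor position as its location.
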(fn NewFunction)

(fn ReceivedNotify
  (params (MeshComp :type Skeletal%20Mesh%20Component%20Object%20Reference) (Animation :type Anim%20Sequence%20Base%20Object%20Reference) (EventReference :type Anim%20Notify%20Event%20Reference%20Structure%20%28by%20ref%29))
  (bind _returnvalue (Math|Random|RandomFloatinRange 0.93 1.07))
  (bind _returnvalue_2 (Components|GetOwner MeshComp))
  (bind _returnvalue_3 (Transformation|GetActorLocation _returnvalue_2))
  (bind (_outhit _returnvalue_4) (Collision|LineTraceByChannel _returnvalue_3 (+ _returnvalue_3 (* (Transformation|GetActorUpVector _returnvalue_2) -2e+02)) "TraceTypeQuery1" false 0 "None"))
  (if _returnvalue_4
    (switch Utilities|FlowControl|Switch|SwitchonEPhysicalSurface (Collision|GetSurfaceType _outhit)
      (:SurfaceType_Default
        (Audio|PlaySoundatLocation "/Game/Resources/SFX/Footsteps/Step3.Step3" "0, 0, 0" "0, 0, 0" 0.4 _returnvalue 0.0 0 0 0 0))
      (:SurfaceType1
        (Audio|PlaySoundatLocation "/Game/Resources/SFX/Footsteps/StepForest1.StepForest1" "0, 0, 0" "0, 0, 0" 0.4 _returnvalue 0.0 0 0 0 0))
      (:SurfaceType2
        (Audio|PlaySoundatLocation "/Game/Resources/SFX/Footsteps/StepMetal2.StepMetal2" "0, 0, 0" "0, 0, 0" 0.8 _returnvalue 0.0 0 0 0 0))
      (:SurfaceType3
        (Audio|PlaySoundatLocation "/Game/Resources/SFX/Footsteps/Step8.Step8" "0, 0, 0" "0, 0, 0" 0.4 _returnvalue 0.0 0 0 0 0))
      (:SurfaceType4
        (Audio|PlaySoundatLocation "/Game/Resources/SFX/Footsteps/waterStep.waterStep" "0, 0, 0" "0, 0, 0" (Math|Random|RandomFloatinRange 0.25 0.35) (Math|Random|RandomFloatinRange 0.9 1.0) 0.0 0 0 0 0))))
  (return false))